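; BP_Ojbect is an actor that provides click-to-move control for a Sedan pawn.
; It enables input from player controller 0 on BeginPlay, and a left click line-traces along the deprojected cursor ray on the Visibility channel.
; The hit location repositions a Target actor, which is passed to the Sedan's PawnMove without checking whether the trace hit.
; A matching PawnMove call for ThirdPersonCharacter is present but never runs.
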(event `self.ReceiveBeginPlay`
  (`self.EnableInput` (`GameplayStatics.GetPlayerController` 0)))

(event `Key|LeftMouseButton`
  (params (Key :type "Key Structure"))
  (bind _target (`self.Target`))
  (bind (_worldlocation _worlddirection) (`PlayerController.DeprojectMousePositionToWorld` (`GameplayStatics.GetPlayerController` 0)))
  (:`Pressed`
    (bind _outhit (`KismetSystemLibrary.LineTraceSingle` _worldlocation (+ _worldlocation (* _worlddirection 1000000.0)) "TraceTypeQuery1"))
    (`self.K2_SetActorLocation` _target (`.Location` (`GameplayStatics.BreakHitResult` _outhit)) false false)
    ;[1 1 1] 车辆目标点跟随
    (`/Game/VehicleBP/Sedan/Sedan.PawnMove` (`self.Sedan`) _target)))

(fn `UserConstructionScript`)